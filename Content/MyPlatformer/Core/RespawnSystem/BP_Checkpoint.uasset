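; Checkpoint actor for the platformer's respawn system that sets the respawn point when its box is overlapped.
; Any overlap sends the arrow component's world location and rotation, plus a self reference, to GM_MyPlatformer through UpdateRespawnPoint.
; It then swaps the button mesh to its alternate material and plays a 2D sound.
; A ReturnToNormal event restores the default material, letting external code reset the checkpoint's look.
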(event OnComponentBeginOverlap(Box)
  (params (OverlappedComponent :type Primitive%20Component%20Object%20Reference) (OtherActor :type Actor%20Object%20Reference) (OtherComp :type Primitive%20Component%20Object%20Reference) (OtherBodyIndex :type Integer) (bFromSweep :type Boolean) (SweepResult :type Hit%20Result%20Structure%20%28by%20ref%29))
  (bind _arrow (Variables|Default|GetArrow))
  (bind _returnvalue (Transformation|GetWorldTransform _arrow))
  (bind _asgm_my_platformer (Utilities|Casting|CastToGM_MyPlatformer (Game|GetGameMode)))
  (Default|UpdateRespawnPoint _asgm_my_platformer (Math|Transform|MakeTransform (.location _returnvalue) (.rotation _returnvalue) "1.000000,1.000000,1.000000") self)
  (Rendering|Material|SetMaterial (Variables|Default|GetSM_Button_A_Push) 0 "/Game/TeachersMarketplace/Assets/Props/Buttons/Button_A/Material/M_Button_A_2.M_Button_A_2")
  (Audio|PlaySound2D (Variables|Default|GetSound) 1.0 1.0 0.0 0 0))

(event Custom|ReturnToNormal
  (Rendering|Material|SetMaterial (Variables|Default|GetSM_Button_A_Push) 0 "/Game/TeachersMarketplace/Assets/Props/Buttons/Button_A/Material/M_Button_A.M_Button_A"))

(event EventBeginPlay)

(event Collision|EventActorBeginOverlap
  (params (OtherActor :type Actor%20Object%20Reference)))

(event EventTick
  (params (DeltaSeconds :type Float%20%28single-precision%29)))

(fn ConstructionScript)