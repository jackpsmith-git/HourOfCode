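; Game mode for a platformer that tracks the player's respawn point and the win moment.
; BeginPlay seeds the respawn transform from a PlayerStart actor.
; UpdateRespawnPoint stores a new transform and checkpoint, first returning any previously active checkpoint to its normal state.
; WinTheGame tells the player's BP_MainCharacter to enter its celebration.
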(event Custom|WinTheGame
  ;[1 1 1] Win The Game
  (bind _asbp_main_character (Utilities|Casting|CastToBP_MainCharacter (Game|GetPlayerCharacter 0)))
  (Default|EnterCelebration _asbp_main_character))

(event EventBeginPlay
  ;[1 1 1] Event Management
  (bind _returnvalue (Actor|GetActorOfClass "/Script/Engine.PlayerStart"))
  (Variables|Default|SetRespawnPoint (Transformation|GetActorTransform _returnvalue)))

(event EventTick
  (params (DeltaSeconds :type Float%20%28single-precision%29))
  ;[1 1 1] Event Management
)

(fn ConstructionScript)

(fn UpdateRespawnPoint
  (params (NewRespawnPoint :type Transform) (CheckpointRef :type BP%20Checkpoint%20Object%20Reference))
  (Utilities|FlowControl|Sequence
    (:then_0
      (if (Utilities|IsValid (Variables|Default|GetCurrent%20Checkpoint%20Ref))
        (Default|ReturntoNormal (Variables|Default|GetCurrent%20Checkpoint%20Ref))))
    (:then_1
      (Variables|Default|SetRespawnPoint NewRespawnPoint)
      (Variables|Default|SetCurrent%20Checkpoint%20Ref CheckpointRef))))